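; Base Blueprint for an actor distribution tool that computes placement for the selected actors.
; CalculateLocation returns a zero vector as a stub for child distribution shapes.
; CalculateRotation keeps the current rotation, faces toward or away from the center, or randomizes it, based on Orientation.
; SetLocation sets the center to the selection's average position, and SetSize takes the first actor's horizontal distance from that center.
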(fn `CalculateLocation`
  (params (Selection :type "Array of Actor Object Reference (by ref)") (ElementID :type Integer))
  (returns (NewLocation :type "Vector Structure"))
  (return (0.0 0.0 0.0)))

(fn `CalculateRotation`
  (params (NewLocation :type "Vector Structure") (CurrentRotation :type "Rotator Structure"))
  (returns (NewRotation :type "Rotator Structure"))
  (bind _location (`self.Location`))
  (switch `/UtilityToolkit/ActorDistributionTool/E_CircleDistributionOrientation` (`self.Orientation`)
    (:`NewEnumerator0`
      (return CurrentRotation))
    (:`NewEnumerator1`
      (return (`KismetMathLibrary.FindLookAtRotation` NewLocation _location)))
    (:`NewEnumerator2`
      (return (`KismetMathLibrary.FindLookAtRotation` _location NewLocation)))
    (:`NewEnumerator3`
      (return (`KismetMathLibrary.RandomRotator` true)))))

(fn `SetLocation`
  (locals (AverageLocation :type "Vector Structure" :default (0.0 0.0 0.0)))
  (bind _returnvalue (`EditorUtilityLibrary.GetSelectionSet`))
  (for _array_element _returnvalue
    (set `local.AverageLocation` (+ (`local.AverageLocation`) (`Actor.K2_GetActorLocation` _array_element))))
  (set `self.Location` (/ (`local.AverageLocation`) (`KismetArrayLibrary.Array_Length` _returnvalue))))

(fn `SetSize`
  (bind _returnvalue (`EditorUtilityLibrary.GetSelectionSet`))
  (if (> (`KismetArrayLibrary.Array_Length` _returnvalue) 0)
    (bind (_returnvalue_x _returnvalue_y) (`KismetMathLibrary.BreakVector` (- (`Actor.K2_GetActorLocation` (`|GetArrayItem` _returnvalue)) (`self.Location`))))
    (set `self.Size` (`KismetMathLibrary.VSize` (`KismetMathLibrary.MakeVector` _returnvalue_x _returnvalue_y)))))