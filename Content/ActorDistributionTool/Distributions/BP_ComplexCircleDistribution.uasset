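; BP_ComplexCircleDistribution is a distribution in the Actor Distribution Tool that computes positions for selected elements along an elliptical arc.
; CalculateLocation spaces elements by ArcAngle divided by the selection count, shifted by AngleOffset.
; Sine and cosine give a flat XY point, with Size multiplied by SizeRatio on X and divided by it on Y.
; That point is rotated by Rotation and added to Location.
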(fn `CalculateLocation`
  (params (Selection :type "Array of Actor Object Reference (by ref)") (ElementID :type Integer))
  (returns (NewLocation :type "Vector Structure"))
  (bind _returnvalue (+ (* ElementID (/ (`self.ArcAngle`) (`KismetArrayLibrary.Array_Length` Selection))) (`self.AngleOffset`)))
  (return (+ (`self.Location`) (`KismetMathLibrary.GreaterGreater_VectorRotator` (`KismetMathLibrary.MakeVector` (* (* (`self.Size`) (`self.SizeRatio`)) (`KismetMathLibrary.Sin` _returnvalue)) (* (/ (`self.Size`) (`self.SizeRatio`)) (`KismetMathLibrary.Cos` _returnvalue))) (`self.Rotation`)))))