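; Geometry Scripting generator actor that builds a hollow sphere shell and bakes it to a static mesh asset.
; Rebuilding boolean-subtracts an inner box-sphere from an outer one using radius, wall thickness and steps settings, then scales UVs.
; Baking overwrites an existing asset, or saves a new one and spawns a baked actor carrying collision profile, materials, settings and generator class.
; Either successful path destroys the generator.
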(event `self.OnRebuildGeneratedMesh`
  (params (TargetMesh :type "DynamicMesh Object Reference"))
  (bind (_meshsettings_radius _meshsettings_wallthickness _meshsettings_steps) (break `/UtilityToolkit/GeometryScripting/S_MeshSettings` (`self.MeshSettings`)))
  (bind (_meshsettings_radius_2 _meshsettings_wallthickness_2 _meshsettings_steps_2) (break `/UtilityToolkit/GeometryScripting/S_MeshSettings` (`self.MeshSettings`)))
  (bind (_meshsettings_radius_3 _meshsettings_wallthickness_3 _meshsettings_steps_3 _meshsettings_uvscale) (break `/UtilityToolkit/GeometryScripting/S_MeshSettings` (`self.MeshSettings`)))
  (bind _returnvalue (`GeometryScriptLibrary_MeshPrimitiveFunctions.AppendSphereBox` TargetMesh (struct) (struct) _meshsettings_radius_2 _meshsettings_steps_2 _meshsettings_steps_2 _meshsettings_steps_2 "Center" null))
  (bind _returnvalue_2 (`self.AllocateComputeMesh`))
  (bind _returnvalue_3 (`GeometryScriptLibrary_MeshPrimitiveFunctions.AppendSphereBox` _returnvalue_2 (struct) (struct) (- _meshsettings_radius _meshsettings_wallthickness) _meshsettings_steps _meshsettings_steps _meshsettings_steps "Center" null))
  (bind _returnvalue_4 (`GeometryScriptLibrary_MeshBooleanFunctions.ApplyMeshBoolean` _returnvalue (struct) _returnvalue_3 (struct) "Subtract" (struct) null))
  (`GeometryScriptLibrary_MeshUVFunctions.ScaleMeshUVs` _returnvalue_4 0 _meshsettings_uvscale (0.0 0.0) null)
  (`self.ReleaseAllComputeMeshes`))

(event `CallBakeToStaticMesh`
  (bind (_assetsettings_meshpath _assetsettings_meshname) (break `/UtilityToolkit/GeometryScripting/S_AssetSettings` (`self.AssetSettings`)))
  (bind _returnvalue (`KismetStringLibrary.Concat_StrStr` _assetsettings_meshpath _assetsettings_meshname))
  (bind _returnvalue_2 (`BaseDynamicMeshComponent.GetDynamicMesh` (`self.DynamicMeshComponent`)))
  (if (`BlueprintPathsLibrary.FileExists` _returnvalue)
    (`self.CopyToExistingStaticMeshAsset` _returnvalue_2 _returnvalue)
    (else
      (`self.CreateNewStaticMeshAsset` _returnvalue_2))))

(event `CreateNewStaticMeshAsset`
  (params (FromDynamicMesh :type "DynamicMesh Object Reference"))
  (bind _dynamicmeshcomponent (`self.DynamicMeshComponent`))
  (bind (_assetsettings_meshpath _assetsettings_meshname) (break `/UtilityToolkit/GeometryScripting/S_AssetSettings` (`self.AssetSettings`)))
  (bind _returnvalue (`GeometryScriptLibrary_CreateNewAssetFunctions.CreateNewStaticMeshAssetFromMesh` FromDynamicMesh (`KismetStringLibrary.Concat_StrStr` _assetsettings_meshpath _assetsettings_meshname) (make `GeometryScriptCreateNewStaticMeshAssetOptions` true true) null)
    (:`Success`
      (bind _returnvalue_2 (`EditorAssetLibrary.SaveLoadedAsset` _returnvalue))
      (if _returnvalue_2
        (bind _returnvalue_3 (`|SpawnActorFromClass` "/UtilityToolkit/GeometryScripting/SM_BakedStaticMeshActor.SM_BakedStaticMeshActor_C" (`self.GetTransform`) "Undefined" "OverrideRootScale" null null))
        (bind _staticmeshcomponent (`StaticMeshActor.StaticMeshComponent` _returnvalue_3))
        (bind _returnvalue_4 (`StaticMeshComponent.SetStaticMesh` _staticmeshcomponent _returnvalue))
        (if _returnvalue_4
          (`PrimitiveComponent.SetCollisionProfileName` _staticmeshcomponent (`PrimitiveComponent.GetCollisionProfileName` _dynamicmeshcomponent) true)
          (`GeometryScriptLibrary_SceneUtilityFunctions.SetComponentMaterialList` _staticmeshcomponent (`MeshComponent.GetMaterials` _dynamicmeshcomponent) null)
          (set `/UtilityToolkit/GeometryScripting/SM_BakedStaticMeshActor.MeshSettings` (`self.MeshSettings`) _returnvalue_3)
          (bind _output_get (set `/UtilityToolkit/GeometryScripting/SM_BakedStaticMeshActor.AssetSettings` (`self.AssetSettings`) _returnvalue_3))
          (setmembers `/UtilityToolkit/GeometryScripting/S_AssetSettings` :`StructRef` _output_get :`GeneratorClass` (`|ConvertAsset` (`GameplayStatics.GetObjectClass` self)))
          (`self.K2_DestroyActor`))))))

(event `CopyToExistingStaticMeshAsset`
  (params (FromDynamicMesh :type "DynamicMesh Object Reference") (AssetPath :type String))
  (bind _returnvalue (`EditorAssetLibrary.LoadAsset` AssetPath))
  (bind _asstatic_mesh (cast `StaticMesh` _returnvalue))
  (`GeometryScriptLibrary_StaticMeshFunctions.CopyMeshToStaticMesh` FromDynamicMesh _asstatic_mesh (make `GeometryScriptCopyMeshToAssetOptions` true true true) (struct) null
    (:`Success`
      (`self.K2_DestroyActor`))))

(fn `BakeToStaticMesh`
  (`self.CallBakeToStaticMesh`))

(fn `UserConstructionScript`
  (`DynamicMeshComponent.EnableComplexAsSimpleCollision` (`self.DynamicMeshComponent`))
  (setmembers `/UtilityToolkit/GeometryScripting/S_AssetSettings` :`StructRef` (`self.AssetSettings`) :`GeneratorClass` (`|ConvertAsset` (`GameplayStatics.GetObjectClass` self))))