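; Distribution Blueprint for the actor distribution tool that places a selection's elements on a Fibonacci-style spiral sphere.
; CalculateLocation maps each ElementID to an evenly stepped height from top to bottom along Y, deriving the ring radius from that height.
; A constant angular step, three Pi minus the square root of SpiralWinding, winds points around that axis.
; The resulting unit-sphere point is scaled by Size and offset by Location.
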(fn `CalculateLocation`
  (params (Selection :type "Array of Actor Object Reference (by ref)") (ElementID :type Integer))
  (returns (NewLocation :type "Vector Structure"))
  (bind _returnvalue (* (- (* (`KismetMathLibrary.GetPI`) 3.0) (`KismetMathLibrary.Sqrt` (`self.SpiralWinding`))) ElementID))
  (bind _returnvalue_2 (- 1.0 (* (/ ElementID (- (`KismetArrayLibrary.Array_Length` Selection) 1)) 2.0)))
  (bind _returnvalue_3 (`KismetMathLibrary.Sqrt` (- 1.0 (* _returnvalue_2 _returnvalue_2))))
  (return (+ (* (`KismetMathLibrary.MakeVector` (* (`KismetMathLibrary.Cos` _returnvalue) _returnvalue_3) _returnvalue_2 (* (`KismetMathLibrary.Sin` _returnvalue) _returnvalue_3)) (`self.Size`)) (`self.Location`))))