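; BP_SnapToSurface is an editor-utility style actor that snaps itself onto nearby surfaces along a configurable direction, shown by an arrow component.
; Snap line-traces on Visibility along the arrow, then moves the actor to the hit and aligns its Z axis to the surface normal.
; The snap runs inside an undo transaction, cancelled on a miss.
; Helper functions randomize the direction, nudge along it, or reset relative location and rotation.
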(fn `Nudge`
  (`self.K2_SetActorLocation` (+ (`self.K2_GetActorLocation`) (* (`SceneComponent.GetForwardVector` (`self.SnapDirectionArrow`)) (`self.NudgeDistance`)))))

(fn `RandomizeDirection`
  (bind _output_get (set `self.SnapDirection` (`KismetMathLibrary.RandomRotator` false)))
  (`SceneComponent.K2_SetRelativeRotation` (`self.SnapDirectionArrow`) _output_get false false))

(fn `ResetLocation`
  (`self.K2_SetActorRelativeLocation` (0.0 0.0 0.0)))

(fn `ResetRotation`
  (`self.K2_SetActorRelativeRotation` (struct)))

(fn `Snap`
  (locals (TransactionID :type Integer :default 0))
  (bind _snapdirectionarrow (`self.SnapDirectionArrow`))
  (bind _returnvalue (`SceneComponent.K2_GetComponentLocation` _snapdirectionarrow))
  (bind _returnvalue_2 (`KismetSystemLibrary.BeginTransaction` "SnapToSurface" "Snap"))
  (set `local.TransactionID` _returnvalue_2)
  (`KismetSystemLibrary.TransactObject` self)
  (bind (_outhit _returnvalue_3) (`KismetSystemLibrary.LineTraceSingle` :`Start` _returnvalue :`End` (+ _returnvalue (* (`SceneComponent.GetForwardVector` _snapdirectionarrow) (`self.MaxSnapDistance`))) :`TraceChannel` "TraceTypeQuery1" :`DrawDebugType` "ForDuration" :`DrawTime` 0.25))
  (if _returnvalue_3
    (bind (_bblockinghit _binitialoverlap _time _distance _location _impactpoint _normal) (`GameplayStatics.BreakHitResult` _outhit))
    (`self.K2_SetActorLocationAndRotation` _location (`KismetMathLibrary.MakeRotFromZ` _normal))
    (`KismetSystemLibrary.EndTransaction`)
    (else
      (`KismetSystemLibrary.CancelTransaction` (`local.TransactionID`)))))

(fn `UserConstructionScript`
  (`SceneComponent.K2_SetRelativeRotation` (`self.SnapDirectionArrow`) (`self.SnapDirection`) false false))