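; 3D grid distribution for the Actor Distribution Tool that computes where each element is placed.
; CalculateLocation turns the element ID into grid indices with integer division and modulo, filling X first, then Y, then stacking layers along Z.
; The indices are scaled by Size and offset by Location.
; SizeX and SizeY bound each layer, while the layer count grows with the ID.
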(fn `CalculateLocation`
  (params (Selection :type "Array of Actor Object Reference (by ref)") (ElementID :type Integer))
  (returns (NewLocation :type "Vector Structure"))
  (bind _sizex (`self.SizeX`))
  (bind _returnvalue (/ ElementID (* (`self.SizeX`) (`self.SizeY`))))
  (bind _returnvalue_2 (- ElementID (* _returnvalue (`self.SizeX`) (`self.SizeY`))))
  (return (+ (* (`KismetMathLibrary.MakeVector` (`KismetMathLibrary.Conv_IntToDouble` (mod _returnvalue_2 _sizex)) (`KismetMathLibrary.Conv_IntToDouble` (/ _returnvalue_2 _sizex)) (`KismetMathLibrary.Conv_IntToDouble` _returnvalue)) (`self.Size`)) (`self.Location`))))