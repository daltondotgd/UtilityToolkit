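; BP_CircleDistribution is an actor distribution tool Blueprint that places a selection of elements along a circle or arc.
; CalculateLocation divides the arc angle by the selection count to get the step, then multiplies it by the element index and adds an angle offset.
; It rotates a Size-length X vector around the Z axis by that angle and adds it to the center location.
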(fn `CalculateLocation`
  (params (Selection :type "Array of Actor Object Reference (by ref)") (ElementID :type Integer))
  (returns (NewLocation :type "Vector Structure"))
  (return (+ (`self.Location`) (`KismetMathLibrary.RotateAngleAxis` (`KismetMathLibrary.MakeVector` (`self.Size`)) (+ (* ElementID (/ (`self.ArcAngle`) (`KismetArrayLibrary.Array_Length` Selection))) (`self.AngleOffset`)) (0.0 0.0 1.0)))))